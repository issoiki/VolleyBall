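; AI controller for BP_AI_Character pawns in a ball game, meant to send the one closest to a predicted impact point and return it after a punch.
; Closest-actor selection compares ball distances but only ever clears ClosestActor, never assigns it; a comment marks the move logic as not working.
; Binding to BP_Ball's punch and landing-prediction events and an AIMoveTo test are unconnected, and BeginPlay is empty.
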(event Custom|MovePosessedActorToPoint
  (params (ImpactPoint :type Vector))
  (bind _returnvalue (Pawn|GetControlledPawn))
  (bind _asbp_ai_character (Utilities|Casting|CastToBP_AI_Character _returnvalue))
  ;[1 1 1] Move closest actor to predicted impact point of ball (not working for now)
  (Default|SetDistancetoBall _asbp_ai_character ImpactPoint)
  (CallFunction|FindClosestActortoPoint)
  ;;[1 1 1] call move to impact point only if own pawn is closest to impact point
  (if (== _asbp_ai_character (Variables|Default|GetClosestActor))
    (Default|MovetoImpactPoint _asbp_ai_character ImpactPoint)))

(event Custom|ReturnToInitPosition
  (params (CharThatPunched :type Character%20Object%20Reference))
  (bind _closestactor (Variables|Default|GetClosestActor))
  ;[1 1 1] Move closest actor to predicted impact point of ball (not working for now)
  (if (== CharThatPunched _closestactor)
    (Default|MovetoInitPosition _closestactor)
    (else
      (Development|PrintString "ERROR: Punched AI is not actor that were moved by Controller"))))

(event EventBeginPlay)

(fn ConstructionScript)

(fn FindClosestActortoPoint
  ;[1 1 1] after loop each AI char knows about closest AI char to ball
  (for _array_element (Variables|Default|GetPossessedActors)
    (if (< (Variables|/Game/Blueprints/AI/BP_AI_Character.BP_AI_Character_C|GetDistanceToBall _array_element) (Variables|/Game/Blueprints/AI/BP_AI_Character.BP_AI_Character_C|GetDistanceToBall (.AsBP%20AI%20Character (Utilities|Casting|CastToBP_AI_Character (Pawn|GetControlledPawn)))))
      (Variables|Default|SetClosestActor 0))))