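; AI-controlled character that hits BP_Ball back toward the PlayerStart location in a ball game.
; When the ball enters its Sphere, it punches it along a slightly scaled-down SuggestProjectileVelocityCustomArc launch vector and plays a jump montage.
; Helper functions store its 2D distance to an impact point, request a move there, or return it to the position saved in the construction script.
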(event OnComponentBeginOverlap(Sphere)
  (params (OverlappedComponent :type Primitive%20Component%20Object%20Reference) (OtherActor :type Actor%20Object%20Reference) (OtherComp :type Primitive%20Component%20Object%20Reference) (OtherBodyIndex :type Integer) (bFromSweep :type Boolean) (SweepResult :type Hit%20Result%20Structure%20%28by%20ref%29))
  (bind _asbp_ball (Utilities|Casting|CastToBP_Ball OtherActor))
  (bind _returnvalue (Actor|GetActorOfClass "/Script/Engine.PlayerStart"))
  (bind _outlaunchvelocity (Game|SuggestProjectileVelocityCustomArc (Transformation|GetActorLocation self) (Transformation|GetActorLocation _returnvalue) 0.0 0.2))
  (Default|Punch _asbp_ball self (* _outlaunchvelocity 0.9) true)
  (Animation|Montage|PlayMontage (Variables|Character|GetMesh) "/Game/Assets/Characters/Mannequins/Animations/Manny/MM_Jump_Montage.MM_Jump_Montage"))

(event EventBeginPlay)

(event Collision|EventActorBeginOverlap
  (params (OtherActor :type Actor%20Object%20Reference)))

(event EventTick
  (params (DeltaSeconds :type Float%20%28single-precision%29)))

(fn ConstructionScript
  (Variables|Default|SetInitPosition (Transformation|GetActorLocation)))

(fn MovetoInitPosition
  (AI|Navigation|SimpleMovetoLocation (AI|GetAIController 0) (Variables|Default|GetInitPosition)))

(fn SetDistancetoBall
  (params (ImpactPoint :type Vector))
  (Variables|Default|SetDistanceToBall (Math|Vector|Distance2D(Vector) ImpactPoint (Transformation|GetActorLocation))))

(fn MovetoImpactPoint
  (params (ImpactPoint :type Vector))
  (AI|Navigation|SimpleMovetoLocation 0 ImpactPoint))