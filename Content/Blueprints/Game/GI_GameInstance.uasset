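; Game instance that keeps success and failure scores across rounds and decides when the game is over.
; AddScore updates both tallies, checks success before failure against a shared score limit, then sets GameStatus and broadcasts RoundEnded.
; If neither limit is reached, it reloads the current level for the next round.
; StartNewGame zeroes the scores and reloads, while GetScores exposes both tallies.
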(fn AddScore
  (params (SuccessScoreToAdd :type Integer) (FailureScoreToAdd :type Integer))
  (Utilities|FlowControl|Sequence
    (:then_0
      (Variables|Default|SetPlayerScoreSuccess (+ SuccessScoreToAdd (Variables|Default|GetPlayerScoreSuccess)))
      (Variables|Default|SetPlayerScoreFailure (+ FailureScoreToAdd (Variables|Default|GetPlayerScoreFailure))))
    (:then_1
      (if (>= (Variables|Default|GetPlayerScoreSuccess) (Variables|Default|GetMaxScoreToFinish))
        (bind _output_get (Variables|Default|SetGameStatus "NewEnumerator1"))
        (Default|CallRoundEnded _output_get)
        (return _output_get)
        (elif (>= (Variables|Default|GetPlayerScoreFailure) (Variables|Default|GetMaxScoreToFinish))
          (bind _output_get_2 (Variables|Default|SetGameStatus "NewEnumerator0"))
          (Default|CallRoundEnded _output_get_2)
          (return _output_get_2)
          (else
            (bind _output_get_3 (Variables|Default|SetGameStatus "NewEnumerator3"))
            (Default|CallRoundEnded _output_get_3)
            (CallFunction|ReloadRound)
            (return _output_get_3)))))))

(fn ReloadRound
  (bind _returnvalue (Game|GetCurrentLevelName true))
  (Game|OpenLevel(byName) (Utilities|String|StringToName _returnvalue)))

(fn GetScores
  (return (Variables|Default|GetPlayerScoreSuccess) (Variables|Default|GetPlayerScoreFailure)))

(fn StartNewGame
  (Variables|Default|SetPlayerScoreFailure 0)
  (Variables|Default|SetPlayerScoreSuccess 0)
  (CallFunction|ReloadRound))