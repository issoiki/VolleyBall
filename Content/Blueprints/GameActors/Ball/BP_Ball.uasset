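; BP_Ball is the physics ball that player and bot punch between court fields, scoring when it overlaps one.
; Punches reset velocity and apply an impulse, with a separate fixed nudge for round start.
; Bot punches broadcast BallPunched; other punches wait briefly, then trace the projectile path and broadcast the predicted landing point.
; Field component tags decide the score sent to GI_GameInstance, with neutral field hits counting against the last puncher.
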(event OnComponentBeginOverlap(Sphere)
  (params (OverlappedComponent :type Primitive%20Component%20Object%20Reference) (OtherActor :type Actor%20Object%20Reference) (OtherComp :type Primitive%20Component%20Object%20Reference) (OtherBodyIndex :type Integer) (bFromSweep :type Boolean) (SweepResult :type Hit%20Result%20Structure%20%28by%20ref%29))
  (bind _gameinstance (Variables|Default|GetGameInstance))
  (bind _charlastpunched (Variables|Default|GetCharLastPunched))
  (bind _gameinstance_2 (Variables|Default|GetGameInstance))
  (switch string (Utilities|String|ToString(Name) (Utilities|Array|Get(acopy) (Variables|/Script/Engine.ActorComponent|GetComponentTags OtherComp)))
    (:PlayerField
      (Development|PrintString "BallOnPlayerField")
      (Default|AddScore _gameinstance_2 0 1))
    (:BotField
      (Development|PrintString "BallOnBotField")
      (Default|AddScore _gameinstance_2 1))
    (:NeutralField
      (Development|PrintString "BallOnNeutralField")
      (Utilities|Casting|CastToBP_PlayerCharacter _charlastpunched
        (:then
          (Default|AddScore _gameinstance 0 1))
        (:CastFailed
          (Utilities|Casting|CastToBP_AI_Character _charlastpunched
            (:then
              (Default|AddScore _gameinstance 1))
            (:CastFailed
              (Development|PrintString "ERROORRR"))))))))

(event Custom|Punch
  (params (CharThatPunched :type Character%20Object%20Reference) (PunchVector :type Vector) (IsBotPunching :type Boolean))
  (Variables|Default|SetCharLastPunched CharThatPunched)
  (Physics|SetPhysicsLinearVelocity (Variables|Default|GetSphereMesh) "0, 0, 0" false "None")
  (if IsBotPunching
    (Physics|AddImpulse (Variables|Default|GetSphereMesh) PunchVector "None" false)
    (Default|CallBallPunched CharThatPunched)
    (else
      (Physics|AddImpulse (Variables|Default|GetSphereMesh) PunchVector "None" false)
      (Utilities|FlowControl|Delay 0.2)
      (CallFunction|PredictImpact))))

(event Custom|StartRoundPunch
  ;[1 1 1] micro punch when round starts
  (Physics|AddImpulse (Variables|Default|GetSphereMesh) "0.000000,500.000000,200.000000" "None" false))

(event EventBeginPlay
  (bind _asgi_game_instance (Utilities|Casting|CastToGI_GameInstance (Game|GetGameInstance)))
  (Variables|Default|SetGameInstance _asgi_game_instance))

(fn ConstructionScript)

(fn PredictImpact
  (bind _spheremesh (Variables|Default|GetSphereMesh))
  (bind _outhit (Class|GameplayStatics|BlueprintPredictProjectilePathbyTraceChannel (Transformation|GetWorldLocation _spheremesh) (Transformation|GetComponentVelocity _spheremesh) true 5e+01 "ECC_WorldStatic" true (Utilities|Array|MakeArray self) "None" 5.0 1e+01 5.0))
  (Default|CallBallLandPredicted (.impactpoint _outhit)))