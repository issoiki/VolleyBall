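; Player controller that manages the HUD, pause menu and end-of-round screen for a player-versus-bot game.
; On BeginPlay it sets game-only input, binds to the GameInstance's round-ended event and shows the main widget with player and bot scores.
; A win or loss, or pressing Escape, pauses the game, opens the result or pause widget and switches to UI-only input with a visible cursor.
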(event Custom|GameEnd
  (params (GameStatus :type E_GameStatus%20Enum :default "NewEnumerator0"))
  (bind _self self)
  (switch Utilities|FlowControl|Switch|SwitchonE_GameStatus GameStatus
    (:NewEnumerator0
      (Game|SetGamePaused true)
      (bind _returnvalue (UserInterface|CreateWidget "/Game/UI/WD_Win.WD_Win_C"))
      (UserInterface|Viewport|AddtoViewport _returnvalue 0)
      (Variables|Default|SetbShowMouseCursor true)
      (Input|SetInputModeUIOnly _self _returnvalue "DoNotLock" true))
    (:NewEnumerator1
      (Game|SetGamePaused true)
      (bind _returnvalue_2 (UserInterface|CreateWidget "/Game/UI/WD_Win.WD_Win_C" 0 true))
      (UserInterface|Viewport|AddtoViewport _returnvalue_2 0)
      (Variables|Default|SetbShowMouseCursor true)
      (Input|SetInputModeUIOnly _self _returnvalue "DoNotLock" false))))

(event EventBeginPlay
  (Utilities|FlowControl|Sequence
    (:then_0
      (Variables|Default|SetbShowMouseCursor false)
      (Input|SetInputModeGameOnly self false))
    (:then_1
      (bind _asgi_game_instance (Utilities|Casting|CastToGI_GameInstance (Game|GetGameInstance)))
      (bind _output_get (Variables|Default|SetGameInstance _asgi_game_instance))
      (EventDispatchers|BindEventtoRoundEnded _output_get (delegate Custom|GameEnd)))
    (:then_2
      (bind (_playerscoresuccess _playerscorefailure) (Default|GetScores (Variables|Default|GetGameInstance)))
      (bind _returnvalue (UserInterface|CreateWidget "/Game/UI/WD_Main.WD_Main_C" 0 _playerscoresuccess _playerscorefailure))
      (bind _output_get_2 (Variables|Default|SetWD_Main _returnvalue))
      (UserInterface|Viewport|AddtoViewport _output_get_2 0))))

(event Input|KeyboardEvents|Escape
  (params (Key :type Key%20Structure :default "None"))
  (:Pressed
    (bind _returnvalue (UserInterface|CreateWidget "/Game/UI/WD_Pause.WD_Pause_C"))
    (UserInterface|Viewport|AddtoViewport _returnvalue 0)
    (Game|SetGamePaused true)
    (Variables|Default|SetbShowMouseCursor true)
    (Input|SetInputModeUIOnly self 0 "DoNotLock" false)))

(fn ConstructionScript)